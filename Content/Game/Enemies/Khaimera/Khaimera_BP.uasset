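; Khaimera enemy Blueprint that handles the UI feedback for its health bar and damage numbers, on top of its parent class.
; On BeginPlay it binds itself to the health bar widget and hides it, then show and hide events toggle its visibility.
; ShowHitNumber spawns an animated hit-number widget at the projected screen position, sets damage and headshot state, and registers it with its world location through StoreHitNumber.
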(event `self.ReceiveBeginPlay`
  (bind _returnvalue (`WidgetComponent.GetUserWidgetObject` (`self.HealthBar`)))
  (`parent.ReceiveBeginPlay`)
  (bind _asenemy_healthbar_bp (cast `/Game/Game/HUD/EnemyHealthbar_BP` _returnvalue))
  (set `/Game/Game/HUD/EnemyHealthbar_BP.Enemy` self _asenemy_healthbar_bp)
  (`Widget.SetVisibility` _returnvalue "Hidden"))

(event `self.ShowHealthBar`
  (`Widget.SetVisibility` (`WidgetComponent.GetUserWidgetObject` (`self.HealthBar`)) "Visible")
  (`parent.ShowHealthBar`))

(event `self.HideHealthBar`
  (`Widget.SetVisibility` (`WidgetComponent.GetUserWidgetObject` (`self.HealthBar`)) "Hidden"))

(event `self.ShowHitNumber`
  (params (Damage :type Integer) (HitLocation :type "Vector Structure") (bHeadshot :type Boolean))
  ;[1 1 1] Draw a Widget on a screen based on C++ property at the class and C++ function with UPROPERTY macro
  (bind _returnvalue (`|CreateWidget` "/Game/Game/HUD/HitNumber_BP.HitNumber_BP_C"))
  (`UserWidget.AddToViewport` _returnvalue 0)
  (`UserWidget.SetPositionInViewport` _returnvalue (`GameplayStatics.ProjectWorldToScreen` (`GameplayStatics.GetPlayerController` 0) HitLocation) true)
  (`self.StoreHitNumber` _returnvalue HitLocation)
  (set `/Game/Game/HUD/HitNumber_BP.HitText` (`KismetTextLibrary.Conv_IntToText` Damage) _returnvalue)
  (set `/Game/Game/HUD/HitNumber_BP.Headshot` bHeadshot _returnvalue)
  (`UserWidget.PlayAnimation` _returnvalue (`/Game/Game/HUD/HitNumber_BP.HitNumberAnimation` _returnvalue) 0.0 1 "Forward" 1.0 false))

(fn `UserConstructionScript`)