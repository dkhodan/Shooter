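; Shooter HUD that draws a dynamic four-arrow crosshair at the screen center during gameplay.
; DrawHUD computes the center from the viewport size and offsets four directional textures outward by the shooter character's spread multiplier times a maximum spread.
; The character reference is cached lazily in DrawHUD by casting the player pawn, since BeginPlay only casts when the reference is already valid.
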(event `self.ReceiveDrawHUD`
  (params (SizeX :type Integer) (SizeY :type Integer))
  (bind (_x _y) (`KismetMathLibrary.BreakVector2D` (`self.CrosshairBaseCenter`)))
  (bind (_x_2 _y_2) (`KismetMathLibrary.BreakVector2D` (`self.CrosshairBaseCenter`)))
  (bind (_x_3 _y_3) (`KismetMathLibrary.BreakVector2D` (`self.CrosshairBaseCenter`)))
  (bind (_x_4 _y_4) (`KismetMathLibrary.BreakVector2D` (`self.CrosshairBaseCenter`)))
  (bind (_x_5 _y_5) (`KismetMathLibrary.BreakVector2D` (`self.CrosshairLocation`)))
  (bind (_x_6 _y_6) (`KismetMathLibrary.BreakVector2D` (`self.ScreenCenter`)))
  ;[1 1 1] Set screencenter and crosshair location
  (set `self.ScreenCenter` (`KismetMathLibrary.MakeVector2D` (`KismetMathLibrary.Conv_IntToDouble` (/ SizeX 2)) (`KismetMathLibrary.Conv_IntToDouble` (/ SizeY 2))))
  (set `self.CrosshairLocation` (`KismetMathLibrary.MakeVector2D` _x_6 _y_6))
  ;[1 1 1] Make sure that ShooterPlayer is valid
  (`/Engine/EditorBlueprintResources/StandardMacros.IsValid` (`self.ShooterCharacter`)
    (:`Is Valid`
      _)
    (:`Is Not Valid`
      (bind _asshooter_character_bp (cast `/Game/Game/Character/ShooterCharacter_BP` (`GameplayStatics.GetPlayerPawn` 0)))
      (set `self.ShooterCharacter` _asshooter_character_bp)))
  ;[1 1 1] Get Spread Multiplier
  (set `self.CrosshairSpreadMultiplier` (`ShooterCharacter.CrosshairSpreadMultiplier` (`self.ShooterCharacter`)))
  (set `self.CrosshairBaseCenter` (`KismetMathLibrary.MakeVector2D` (- _x_5 (`self.CrosshairHalfWidth`)) (- _y_5 (`self.CrosshairHalfHeight`))))
  ;[1 1 1] Set Crosshair at the screen
  (`self.DrawTexture` "/Game/Game/Assets/Textures/Crosshairs/Crosshair_Quad_9_Bottom.Crosshair_Quad_9_Bottom" _x_2 (+ _y_2 (* (`self.CrosshairSpreadMultiplier`) (`self.CrosshairSpreadMax`))) 64.0 64.0 0.0 0.0 1.0 1.0)
  (`self.DrawTexture` "/Game/Game/Assets/Textures/Crosshairs/Crosshair_Quad_9_Top.Crosshair_Quad_9_Top" _x_3 (- _y_3 (* (`self.CrosshairSpreadMultiplier`) (`self.CrosshairSpreadMax`))) 64.0 64.0 0.0 0.0 1.0 1.0)
  (`self.DrawTexture` "/Game/Game/Assets/Textures/Crosshairs/Crosshair_Quad_9_Left.Crosshair_Quad_9_Left" (- _x_4 (* (`self.CrosshairSpreadMultiplier`) (`self.CrosshairSpreadMax`))) _y_4 64.0 64.0 0.0 0.0 1.0 1.0)
  (`self.DrawTexture` "/Game/Game/Assets/Textures/Crosshairs/Crosshair_Quad_9_Right.Crosshair_Quad_9_Right" (+ _x (* (`self.CrosshairSpreadMultiplier`) (`self.CrosshairSpreadMax`))) _y 64.0 64.0 0.0 0.0 1.0 1.0))

(event `self.ReceiveBeginPlay`
  ;[1 1 1] Get Shooter Character Reference
  (`/Engine/EditorBlueprintResources/StandardMacros.IsValid` (`self.ShooterCharacter`)
    (:`Is Valid`
      (bind _asshooter_character_bp (cast `/Game/Game/Character/ShooterCharacter_BP` (`GameplayStatics.GetPlayerPawn` 0)))
      (set `self.ShooterCharacter` _asshooter_character_bp))))

(fn `UserConstructionScript`)